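; Lobby player controller that displays the pre-game lobby UI.
; It enables input on BeginPlay and exposes events for the lobby, ready-status and countdown widgets, each created for the passed-in controller.
; The lobby and ready events refresh by removing existing top-level instances and recreating the widget with new player counts.
; The timer event simply adds a TimerBeforeGame widget without clearing previous ones.
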(event `self.ReceiveBeginPlay`
  (`self.EnableInput` self))

(event `UiLobby`
  (params (PcLobby :type "/Game/Blueprint/PlayerController/PC_Lobby Object Reference") (NumberOfPlayers :type Integer))
  (bind _foundwidgets (`WidgetBlueprintLibrary.GetAllWidgetsOfClass` "/Game/Widget/LobbyWidget.LobbyWidget_C"))
  (for _array_element _foundwidgets
    (`Widget.RemoveFromParent` _array_element))
  (bind _returnvalue (`|CreateWidget` "/Game/Widget/LobbyWidget.LobbyWidget_C" PcLobby NumberOfPlayers))
  (`UserWidget.AddToViewport` _returnvalue 0))

(event `ReadyLobby`
  (params (PcLobby :type "/Game/Blueprint/PlayerController/PC_Lobby Object Reference") (TotalPlayers :type Integer) (ReadyPlayers :type Integer))
  (bind _foundwidgets (`WidgetBlueprintLibrary.GetAllWidgetsOfClass` "/Game/Widget/ReadyInLobby.ReadyInLobby_C"))
  (for _array_element _foundwidgets
    (`Widget.RemoveFromParent` _array_element))
  (bind _returnvalue (`|CreateWidget` "/Game/Widget/ReadyInLobby.ReadyInLobby_C" PcLobby TotalPlayers ReadyPlayers))
  (`UserWidget.AddToViewport` _returnvalue 0))

(event `TimerLobby`
  (params (`Pc Lobby` :type "/Game/Blueprint/PlayerController/PC_Lobby Object Reference"))
  (bind _returnvalue (`|CreateWidget` "/Game/Widget/TimerBeforeGame.TimerBeforeGame_C" `Pc Lobby`))
  (`UserWidget.AddToViewport` _returnvalue 0))

(fn `UserConstructionScript`)