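; Lobby game mode that tracks joining players and moves the match to ThirdPersonMap once everyone is ready.
; PostLogin stores each controller and updates the player count, which UI events push to PC_Lobby.
; CheckReady refreshes each controller's lobby display; when all are ready, it starts their timers.
; After a short delay, it disables input, clears widgets and runs servertravel, all nested inside the per-player loop.
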(event `self.K2_PostLogin`
  (params (NewPlayer :type "PlayerController Object Reference"))
  (bind _new_player (`self.New Player`))
  (`KismetArrayLibrary.Array_Add` _new_player NewPlayer)
  (bind _output_get (set `self.NbOfPlayers` (`KismetArrayLibrary.Array_Length` _new_player)))
  (`KismetSystemLibrary.PrintString` (`KismetStringLibrary.Conv_IntToString` _output_get) true true (struct :`R` 1.0 :`B` 0.943358 :`A` 1.0) 10.0))

(event `CheckReady`
  (params (NbPlayersReady :type Integer))
  (bind _nbofplayers (`self.NbOfPlayers`))
  (for _array_element (`self.New Player`)
    (bind _aspc_lobby (cast `/Game/Blueprint/PlayerController/PC_Lobby` _array_element))
    (`/Engine/EditorBlueprintResources/StandardMacros.IsValid` _aspc_lobby
      (:`Is Valid`
        (`/Game/Blueprint/PlayerController/PC_Lobby.ReadyLobby` _aspc_lobby _aspc_lobby _nbofplayers NbPlayersReady)
        (`/Game/Blueprint/PlayerController/PC_Lobby.UiLobby` _aspc_lobby _aspc_lobby _nbofplayers)
        (if (== NbPlayersReady (`self.NbOfPlayers`))
          (for _array_element_2 (`self.New Player`)
            (bind _aspc_lobby_2 (cast `/Game/Blueprint/PlayerController/PC_Lobby` _array_element_2))
            (`/Game/Blueprint/PlayerController/PC_Lobby.TimerLobby` _aspc_lobby_2 _aspc_lobby_2))
          (`KismetSystemLibrary.Delay` 5.0)
          (for _array_element_3 (`self.New Player`)
            (bind _aspc_lobby_3 (cast `/Game/Blueprint/PlayerController/PC_Lobby` _array_element_3))
            (`self.DisableInput` _aspc_lobby_3 _aspc_lobby_3)
            (`WidgetLayoutLibrary.RemoveAllWidgets`)
            (`KismetSystemLibrary.ExecuteConsoleCommand` (`KismetStringLibrary.Concat_StrStr` "servertravel" "/Game/Maps/ThirdPersonMap") _array_element_3)))))))

(event `CreateUiNbOfPlayers`
  (params (PlayerController :type "PlayerController Object Reference"))
  (bind _aspc_lobby (cast `/Game/Blueprint/PlayerController/PC_Lobby` PlayerController))
  (`/Game/Blueprint/PlayerController/PC_Lobby.UiLobby` _aspc_lobby _aspc_lobby (`self.NbOfPlayers`)))

(event `CreateUIReadyPlayers`
  (params (PlayerController :type "PlayerController Object Reference"))
  (bind _aspc_lobby (cast `/Game/Blueprint/PlayerController/PC_Lobby` PlayerController))
  (`/Game/Blueprint/PlayerController/PC_Lobby.ReadyLobby` _aspc_lobby _aspc_lobby (`self.NbOfPlayers`) (`self.PlayersReady`)))

(fn `UserConstructionScript`)