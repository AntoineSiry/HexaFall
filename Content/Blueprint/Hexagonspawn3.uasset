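; Spawner actor that lays out a line of alternating Hexagonspawn1 and Hexagonspawn2 actors when play begins.
; On BeginPlay a loop steps from the Scene component's world location along world X at a fixed spacing, spawning one actor per step.
; A FlipFlop inside the loop switches between the two classes on each iteration, starting with Hexagonspawn1.
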(event `self.ReceiveBeginPlay`
  (for _index (range 11)
    (set `self.Location` (+ (`SceneComponent.K2_GetComponentLocation` (`self.Scene`)) (`KismetMathLibrary.MakeVector` (* _index 150))))
    (`/Engine/EditorBlueprintResources/StandardMacros.FlipFlop`
      (:`A`
        (`|SpawnActorFromClass` "/Game/Blueprint/Hexagonspawn1.Hexagonspawn1_C" (`KismetMathLibrary.MakeTransform` (`self.Location`)) "Undefined" "OverrideRootScale" null null))
      (:`B`
        (`|SpawnActorFromClass` "/Game/Blueprint/Hexagonspawn2.Hexagonspawn2_C" (`KismetMathLibrary.MakeTransform` (`self.Location`)) "Undefined" "OverrideRootScale" null null)))))

(fn `UserConstructionScript`)