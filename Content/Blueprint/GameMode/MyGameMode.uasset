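; Game mode that centralizes item abilities, item spawning and player UI for a hexagon-based game with multiple players.
; Its events spawn random items at a random hexagon, roll an item number, and apply a big jump or temporary flying gravity effect.
; GetPlayerID stores a character's index among all third-person characters, which the UI events use to route item and elimination displays to that player's controller.
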(event `GetPlayerID`
  (params (ThirdPersonChar :type "/Game/Blueprint/BP_ThirdPersonCharacter Object Reference"))
  (bind _outactors (`GameplayStatics.GetAllActorsOfClass` "/Game/Blueprint/BP_ThirdPersonCharacter.BP_ThirdPersonCharacter_C"))
  (for (_array_element _array_index) _outactors
    (if (== _array_element ThirdPersonChar)
      (set `self.PlayerID` _array_index))))

(event `GetRandomHexagonArray`
  (params (HexagonArray :type "Array of /Game/Blueprint/BlueHexagones/Hexagon Object Reference") (Hexa3 :type "/Game/Blueprint/BlueHexagones/Hexagonspawn3 Object Reference"))
  (`/Game/Blueprint/BlueHexagones/Hexagonspawn3.SpawnRandomItems` Hexa3 (`self.K2_GetActorLocation` (`KismetArrayLibrary.Array_Random` HexagonArray))))

(event `SetGravityForItem`
  (params (CharacterMovement :type "CharacterMovementComponent Object Reference") (ThirdPersonCharacterREF :type "/Game/Blueprint/BP_ThirdPersonCharacter Object Reference") (SkeletalMesh :type "SkeletalMeshComponent Object Reference"))
  (`self.K2_SetActorLocation` ThirdPersonCharacterREF (+ (`self.K2_GetActorLocation` ThirdPersonCharacterREF) (0.0 0.0 100.0)) false false)
  (`CharacterMovementComponent.SetMovementMode` CharacterMovement "MOVE_Flying" 0)
  (`MovementComponent.StopMovementImmediately` CharacterMovement)
  (set `/Game/Blueprint/BP_ThirdPersonCharacter.CanUseCapacity` true ThirdPersonCharacterREF)
  (`KismetSystemLibrary.Delay` 2.0)
  (`CharacterMovementComponent.SetMovementMode` CharacterMovement "MOVE_Walking" 0))

(event `SetBigJump`
  (params (ThirdPersonCharacterREF :type "/Game/Blueprint/BP_ThirdPersonCharacter Object Reference"))
  (`Character.LaunchCharacter` ThirdPersonCharacterREF (0.0 0.0 2000.0) false false)
  (set `/Game/Blueprint/BP_ThirdPersonCharacter.CanUseCapacity` true ThirdPersonCharacterREF))

(event `RandomNumberForItems`
  (bind _returnvalue (`KismetMathLibrary.RandomIntegerInRange` 0 1))
  (switch `int` _returnvalue
    (:`0`
      (set `self.NumberOfTheItem` _returnvalue))
    (:`1`
      (set `self.NumberOfTheItem` _returnvalue))))

(event `CreateUIItems`
  (bind _asmy_player_controller (cast `/Game/Blueprint/PlayerController/MyPlayerController` (`GameplayStatics.GetPlayerController` (`self.PlayerID`))))
  (`/Game/Blueprint/PlayerController/MyPlayerController.UiItems` _asmy_player_controller (`self.NumberOfTheItem`)))

(event `CreateUiElimination`
  (bind _asmy_player_controller (cast `/Game/Blueprint/PlayerController/MyPlayerController` (`GameplayStatics.GetPlayerController` (`self.PlayerID`))))
  (`/Game/Blueprint/PlayerController/MyPlayerController.UiElimination` _asmy_player_controller))

(fn `UserConstructionScript`)