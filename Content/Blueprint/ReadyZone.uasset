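; ReadyZone is a lobby trigger volume that marks third-person characters as ready while they stand inside it.
; Box overlap begin and end events set the character's Ready flag and adjust a running NbReady count.
; Each change calls CheckReady, which prints the count on screen and forwards it to the GM_Lobby game mode's CheckReady.
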(event `self.Box.OnComponentBeginOverlap`
  (params (OverlappedComponent :type "PrimitiveComponent Object Reference") (OtherActor :type "Actor Object Reference") (OtherComp :type "PrimitiveComponent Object Reference") (OtherBodyIndex :type Integer) (bFromSweep :type Boolean) (SweepResult :type "HitResult Structure (by ref)"))
  (bind _asbp_third_person_character (cast `/Game/Blueprint/BP_ThirdPersonCharacter` OtherActor))
  (set `/Game/Blueprint/BP_ThirdPersonCharacter.Ready?` true _asbp_third_person_character)
  (set `self.NbReady` (+ (`self.NbReady`) 1))
  (`self.CheckReady`))

(event `self.Box.OnComponentEndOverlap`
  (params (OverlappedComponent :type "PrimitiveComponent Object Reference") (OtherActor :type "Actor Object Reference") (OtherComp :type "PrimitiveComponent Object Reference") (OtherBodyIndex :type Integer))
  (bind _asbp_third_person_character (cast `/Game/Blueprint/BP_ThirdPersonCharacter` OtherActor))
  (set `/Game/Blueprint/BP_ThirdPersonCharacter.Ready?` false _asbp_third_person_character)
  (set `self.NbReady` (- (`self.NbReady`) 1))
  (`self.CheckReady`))

(event `CheckReady`
  (bind _nbready (`self.NbReady`))
  (bind _asgm_lobby (cast `/Game/Blueprint/GameMode/GM_Lobby` (`GameplayStatics.GetGameMode`)))
  (`KismetSystemLibrary.PrintString` (`KismetStringLibrary.Conv_IntToString` _nbready) true true (struct :`R` 1.0 :`G` 0.8645 :`A` 1.0) 10.0)
  (`/Game/Blueprint/GameMode/GM_Lobby.CheckReady` _asgm_lobby _nbready))

(fn `UserConstructionScript`)