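; Spawner actor that lays out a row of eleven evenly spaced hexagon sub-spawners along X on BeginPlay.
; A FlipFlop alternates between Hexagonspawn1 and Hexagonspawn2, passing its Color to each.
; Each Hexagonspawn1's hexagon array goes to MyGameMode's GetRandomHexagonArray along with a reference to this actor.
; A SpawnRandomItems event spawns a RandomObject at a supplied location.
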(event `self.ReceiveBeginPlay`
  (bind _color (`self.Color`))
  (for _index (range 11)
    (set `self.Location` (+ (`SceneComponent.K2_GetComponentLocation` (`self.Scene`)) (`KismetMathLibrary.MakeVector` (* _index 150))))
    (`/Engine/EditorBlueprintResources/StandardMacros.FlipFlop`
      (:`A`
        (bind _returnvalue (`|SpawnActorFromClass` "/Game/Blueprint/BlueHexagones/Hexagonspawn1.Hexagonspawn1_C" (`KismetMathLibrary.MakeTransform` (`self.Location`)) "Undefined" "OverrideRootScale" null _color null))
        (bind _asmy_game_mode (cast `/Game/Blueprint/GameMode/MyGameMode` (`GameplayStatics.GetGameMode`)))
        (`/Game/Blueprint/GameMode/MyGameMode.GetRandomHexagonArray` _asmy_game_mode (`/Game/Blueprint/BlueHexagones/Hexagonspawn1.HexagonArray` _returnvalue) self))
      (:`B`
        (`|SpawnActorFromClass` "/Game/Blueprint/BlueHexagones/Hexagonspawn2.Hexagonspawn2_C" (`KismetMathLibrary.MakeTransform` (`self.Location`)) "Undefined" "OverrideRootScale" null _color null)))))

(event `SpawnRandomItems`
  (params (LocToSpawn :type "Vector Structure"))
  (`|SpawnActorFromClass` "/Game/Blueprint/RandomObject.RandomObject_C" (`KismetMathLibrary.MakeTransform` LocToSpawn) "Undefined" "OverrideRootScale" null null))

(fn `UserConstructionScript`)