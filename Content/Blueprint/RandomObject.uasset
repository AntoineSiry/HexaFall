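; RandomObject is a floating pickup that grants the third-person character a random item capacity on contact.
; A Levitate timeline started on BeginPlay bobs the object by adding a local offset on each update.
; When the character overlaps the sphere, it enables CanUseCapacity, asks MyGameMode to roll random item numbers, triggers player 0's item UI, then destroys itself.
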(event `self.ReceiveBeginPlay`
  (bind (_direction _updown) (`Timeline|Levitate`)
    (:`Update`
      (`SceneComponent.K2_AddLocalOffset` (`self.Object`) _updown false false))))

(event `self.Sphere.OnComponentBeginOverlap`
  (params (OverlappedComponent :type "PrimitiveComponent Object Reference") (OtherActor :type "Actor Object Reference") (OtherComp :type "PrimitiveComponent Object Reference") (OtherBodyIndex :type Integer) (bFromSweep :type Boolean) (SweepResult :type "HitResult Structure (by ref)"))
  (bind _asbp_third_person_character (cast `/Game/Blueprint/BP_ThirdPersonCharacter` OtherActor))
  (set `self.ThirdPersonCHaracterREF` _asbp_third_person_character)
  (set `/Game/Blueprint/BP_ThirdPersonCharacter.CanUseCapacity` true _asbp_third_person_character)
  (`self.GetRandomNumbersForItems`)
  (`self.CreateWidget`)
  (`self.K2_DestroyActor`))

(event `GetRandomNumbersForItems`
  (bind _asmy_game_mode (cast `/Game/Blueprint/GameMode/MyGameMode` (`GameplayStatics.GetGameMode`)))
  (`/Game/Blueprint/GameMode/MyGameMode.RandomNumberForItems` _asmy_game_mode))

(event `CreateWidget`
  (bind _asbp_third_person_character (cast `/Game/Blueprint/BP_ThirdPersonCharacter` (`GameplayStatics.GetPlayerPawn` 0)))
  (`/Game/Blueprint/BP_ThirdPersonCharacter.UiItems` _asbp_third_person_character))

(fn `UserConstructionScript`)