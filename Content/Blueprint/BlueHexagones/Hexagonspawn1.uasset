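; Hexagonspawn1 is a spawner Blueprint that builds a straight row of Hexagon actors when play begins.
; A loop spawns eleven hexagons from the spawner's scene location, evenly spaced along the world Y axis, and stores each in an array.
; A second pass over that array applies the Color material to the first material slot of every hexagon's mesh.
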(event `self.ReceiveBeginPlay`
  (for _index (range 11)
    (bind _output_get (set `self.Location` (+ (`SceneComponent.K2_GetComponentLocation` (`self.Scene`)) (`KismetMathLibrary.MakeVector` 0.0 (* _index 160)))))
    (bind _returnvalue (`|SpawnActorFromClass` "/Game/Blueprint/BlueHexagones/Hexagon.Hexagon_C" (`KismetMathLibrary.MakeTransform` _output_get) "Undefined" "OverrideRootScale" null null))
    (bind _output_get_2 (set `self.Hexagon1` _returnvalue))
    (`KismetArrayLibrary.Array_Add` (`self.HexagonArray`) _output_get_2))
  (for _array_element (`self.HexagonArray`)
    (`PrimitiveComponent.SetMaterial` (`/Game/Blueprint/BlueHexagones/Hexagon.Hexagon` _array_element) 0 (`self.Color`))))

(fn `UserConstructionScript`)