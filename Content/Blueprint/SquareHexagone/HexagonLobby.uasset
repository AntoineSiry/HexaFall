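; Lobby hexagon tile that sinks, fades out and turns non-solid when a third-person character steps on it, then restores itself.
; A Box overlap passes a DoOnce into a delayed sequence that offsets the tile, toggles Hexagon collision and resets the gate after restoring.
; Looping function-name timers step the material's Appearance parameter down or up and set a high emissive multiplier, clearing themselves at either limit.
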(event `self.ReceiveBeginPlay`
  (`PrimitiveComponent.SetMaterial` (`self.Hexagon`) 0 (`self.Color`)))

(event `self.Box.OnComponentBeginOverlap`
  (params (OverlappedComponent :type "PrimitiveComponent Object Reference") (OtherActor :type "Actor Object Reference") (OtherComp :type "PrimitiveComponent Object Reference") (OtherBodyIndex :type Integer) (bFromSweep :type Boolean) (SweepResult :type "HitResult Structure (by ref)"))
  (bind _hexagon (`self.Hexagon`))
  (cast `/Game/Blueprint/BP_ThirdPersonCharacter` OtherActor)
  (`/Engine/EditorBlueprintResources/StandardMacros.DoOnce` false :!label _label
    (:`Completed`
      (`self.K2_AddActorLocalOffset` (0.0 0.0 -5.0))
      (`KismetSystemLibrary.Delay` 0.2)
      (`self.Dissapear`)
      (`KismetSystemLibrary.Delay` 0.3)
      (`PrimitiveComponent.SetCollisionEnabled` _hexagon "NoCollision")
      (`KismetSystemLibrary.Delay` 1.5)
      (`self.K2_AddActorLocalOffset` (0.0 0.0 5.0))
      (`self.Appear`)
      (`PrimitiveComponent.SetCollisionEnabled` _hexagon "QueryAndPhysics")
      (goto _label :!via `Reset`))))

(event `Appear`
  (`KismetSystemLibrary.K2_SetTimer` null "HexagonAppearance" 0.01 true))

(event `Dissapear`
  (`KismetSystemLibrary.K2_SetTimer` null "HexagonDissapearance" 0.01 true))

(fn `HexagonAppearance`
  (bind _returnvalue (+ (`self.Appearance`) 0.01))
  (bind _returnvalue_2 (`PrimitiveComponent.CreateDynamicMaterialInstance` (`self.Hexagon`) 0 null "None"))
  (`MaterialInstanceDynamic.SetScalarParameterValue` _returnvalue_2 "Appearance" _returnvalue)
  (`MaterialInstanceDynamic.SetScalarParameterValue` _returnvalue_2 "Emmisive_Mult" 10000.0)
  (bind _output_get (set `self.Appearance` _returnvalue))
  (if (>= _output_get 1.0)
    (`KismetSystemLibrary.K2_ClearTimer` null "HexagonAppearance")))

(fn `HexagonDissapearance`
  (bind _returnvalue (- (`self.Appearance`) 0.01))
  (bind _returnvalue_2 (`PrimitiveComponent.CreateDynamicMaterialInstance` (`self.Hexagon`) 0 null "None"))
  (`MaterialInstanceDynamic.SetScalarParameterValue` _returnvalue_2 "Appearance" _returnvalue)
  (`MaterialInstanceDynamic.SetScalarParameterValue` _returnvalue_2 "Emmisive_Mult" 10000.0)
  (bind _output_get (set `self.Appearance` _returnvalue))
  (if (<= _output_get 0.0)
    (`KismetSystemLibrary.K2_ClearTimer` null "HexagonDissapearance")))

(fn `UserConstructionScript`)